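; BP_Tunnel is an endless-runner tunnel segment with a rotating holed wall that the player must pass.
; Passing its trigger asks TunnelSpawner for a new segment, destroys this one, adds score and randomly spawns a health pack and enemy ahead.
; Wall hits damage the player and shake the camera, then recycle the segment or show restart on death; bullets are destroyed.
; RandomizeWall and RandomizeEnemy provide randomization but are not called here.
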(event OnComponentBeginOverlap(TriggerZone)
  (params (OverlappedComponent :type Primitive%20Component%20Object%20Reference) (OtherActor :type Actor%20Object%20Reference) (OtherComp :type Primitive%20Component%20Object%20Reference) (OtherBodyIndex :type Integer) (bFromSweep :type Boolean) (SweepResult :type Hit%20Result%20Structure%20%28by%20ref%29))
  (bind _returnvalue (Game|Player|GetPlayerPawn 0))
  (bind _returnvalue_2 (Game|Player|GetPlayerPawn 0))
  (bind _returnvalue_3 (Transformation|GetActorLocation _returnvalue))
  (bind _returnvalue_4 (Transformation|GetActorLocation _returnvalue_2))
  (bind _asbp_player (Utilities|Casting|CastToBP_Player OtherActor))
  (Default|SpawnTunnelatSpawnPoint (Variables|Default|GetTunnelSpawner))
  (Actor|DestroyActor)
  (bind _output_get (Variables|/Game/InfiniteMatrix/Blueprints/BP_Player.BP_Player_C|SetScoreValue _asbp_player (+ 2 (Variables|/Game/InfiniteMatrix/Blueprints/BP_Player.BP_Player_C|GetScoreValue _asbp_player))))
  (Rendering|Components|TextRender|SetText (Variables|/Game/InfiniteMatrix/UI/WBP_Score.WBP_Score_C|GetScore (Variables|/Game/InfiniteMatrix/Blueprints/BP_Player.BP_Player_C|GetScoreWidget _asbp_player)) (Utilities|Text|ToText(Integer) _output_get))
  (if (== 0 (Math|Random|RandomIntegerinRange 0 1))
    (bind _returnvalue_5 (Game|SpawnActorfromClass "/Game/Blueprints/BP_HealthPack.BP_HealthPack_C" (Math|Transform|MakeTransform (Math|Vector|MakeVector (+ 4e+02 (.x _returnvalue_3)) (+ (Math|Random|RandomFloatinRange -5e+01 0.0) (.y _returnvalue_3)) (+ (.z _returnvalue_3) (Math|Random|RandomFloatinRange -5e+01 5e+01))) "0, 0, 0" "1.000000,1.000000,1.000000") "Undefined" "MultiplyWithRoot" 0 0))
    (Variables|Default|SetNewestHealthPack _returnvalue_5)
    (bind _returnvalue_6 (Game|SpawnActorfromClass "/Game/Blueprints/BP_Enemy.BP_Enemy_C" (Math|Transform|MakeTransform (Math|Vector|MakeVector (+ 6e+02 (.x _returnvalue_4)) (+ (Math|Random|RandomFloatinRange 0.0 75.0) (.y _returnvalue_4)) (+ (.z _returnvalue_4) (Math|Random|RandomFloatinRange -75.0 75.0))) "0, 0, 0" "1.000000,1.000000,1.000000") "Undefined" "MultiplyWithRoot" 0 0))
    (Variables|Default|SetNewestEnemy _returnvalue_6)))

(event OnComponentHit(WallMesh)
  (params (HitComponent :type Primitive%20Component%20Object%20Reference) (OtherActor :type Actor%20Object%20Reference) (OtherComp :type Primitive%20Component%20Object%20Reference) (NormalImpulse :type Vector :default "0, 0, 0") (Hit :type Hit%20Result%20Structure%20%28by%20ref%29))
  (bind _asbp_player (Utilities|Casting|CastToBP_Player OtherActor)
    (:then
      (bind _output_get (Variables|/Game/InfiniteMatrix/Blueprints/BP_Player.BP_Player_C|SetHealthValue _asbp_player (- (Variables|/Game/InfiniteMatrix/Blueprints/BP_Player.BP_Player_C|GetHealthValue _asbp_player) 1)))
      (Rendering|Components|TextRender|SetText (Variables|/Game/InfiniteMatrix/UI/WBP_Health.WBP_Health_C|GetHealth (Variables|/Game/InfiniteMatrix/Blueprints/BP_Player.BP_Player_C|GetHealthWidget _asbp_player)) (Utilities|Text|ToText(Integer) _output_get))
      (Camera|PlayWorldCameraShake "/Game/Blueprints/BP_Camera_Shake.BP_Camera_Shake_C" (Transformation|GetActorLocation (Game|Player|GetPlayerPawn 0)) 0.0 1e+03)
      (if (> _output_get 0)
        (Actor|DestroyActor)
        (Default|SpawnTunnelatSpawnPoint (Variables|Default|GetTunnelSpawner))
        (else
          (Variables|/Game/InfiniteMatrix/Blueprints/BP_Player.BP_Player_C|SetIsDead _asbp_player true)
          (Default|DisplayRestart _asbp_player))))
    (:CastFailed
      (bind _asbp_bullet (Utilities|Casting|CastToBP_Bullet OtherActor))
      (Actor|DestroyActor _asbp_bullet))))

(event OnComponentBeginOverlap(WallMesh)
  (params (OverlappedComponent :type Primitive%20Component%20Object%20Reference) (OtherActor :type Actor%20Object%20Reference) (OtherComp :type Primitive%20Component%20Object%20Reference) (OtherBodyIndex :type Integer) (bFromSweep :type Boolean) (SweepResult :type Hit%20Result%20Structure%20%28by%20ref%29))
  (bind _asbp_bullet (Utilities|Casting|CastToBP_Bullet OtherActor))
  (Actor|DestroyActor _asbp_bullet))

(event EventBeginPlay)

(event EventTick
  (params (DeltaSeconds :type Float%20%28single-precision%29))
  (Transformation|AddLocalRotation (Variables|Default|GetWallMesh) (Math|Rotator|MakeRotator (* DeltaSeconds (Variables|Default|GetRotateSpeed)) 0.0 0.0) false false))

(fn ConstructionScript)

(fn RandomizeWall
  (Components|StaticMesh|SetStaticMesh (Variables|Default|GetWallMesh) (Utilities|Select :Index (Math|Random|RandomIntegerinRange 0 3) :Option%200 "/Game/InfiniteMatrix/Meshes/SM_Hole_01.SM_Hole_01" :Option%201 "/Game/InfiniteMatrix/Meshes/SM_Hole_02.SM_Hole_02" :Option%202 "/Game/InfiniteMatrix/Meshes/SM_Hole_03.SM_Hole_03" :Option%203 "/Game/InfiniteMatrix/Meshes/SM_Hole_04.SM_Hole_04"))
  (Transformation|AddLocalRotation (Variables|Default|GetWallMesh) (Math|Rotator|MakeRotator (Math|Random|RandomFloatinRange 0.0 3.6e+02) 0.0 0.0) false false))

(fn RandomizeEnemy
  (bind _returnvalue (Game|Player|GetPlayerPawn 0))
  (bind _returnvalue_2 (Transformation|GetActorLocation _returnvalue))
  (if (== 0 (Math|Random|RandomIntegerinRange 0 0))
    (Game|SpawnActorfromClass "/Game/Blueprints/BP_HealthPack.BP_HealthPack_C" (Math|Transform|MakeTransform (Math|Vector|MakeVector (+ 2e+02 (.x _returnvalue_2)) (+ (Math|Random|RandomFloatinRange -2e+01 2e+01) (.y _returnvalue_2)) (+ (.z _returnvalue_2) (Math|Random|RandomFloatinRange -2e+01 2e+01))) "0, 0, 0" "1.000000,1.000000,1.000000") "Undefined" "MultiplyWithRoot" 0 0)))