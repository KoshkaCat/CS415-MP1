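; BP_Enemy is a short-lived hazard actor that damages the player on contact and destroys itself three seconds after spawning.
; When its Enemy component hits BP_Player, it decrements the player's health, writes the new value straight into the health widget, plays a camera shake and destroys itself.
; If health drops below one, it marks the player dead and calls the player's restart display.
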(event OnComponentHit(Enemy)
  (params (HitComponent :type Primitive%20Component%20Object%20Reference) (OtherActor :type Actor%20Object%20Reference) (OtherComp :type Primitive%20Component%20Object%20Reference) (NormalImpulse :type Vector :default "0, 0, 0") (Hit :type Hit%20Result%20Structure%20%28by%20ref%29))
  (bind _asbp_player (Utilities|Casting|CastToBP_Player OtherActor))
  (bind _output_get (Variables|/Game/InfiniteMatrix/Blueprints/BP_Player.BP_Player_C|SetHealthValue _asbp_player (- (Variables|/Game/InfiniteMatrix/Blueprints/BP_Player.BP_Player_C|GetHealthValue _asbp_player) 1)))
  (Rendering|Components|TextRender|SetText (Variables|/Game/InfiniteMatrix/UI/WBP_Health.WBP_Health_C|GetHealth (Variables|/Game/InfiniteMatrix/Blueprints/BP_Player.BP_Player_C|GetHealthWidget _asbp_player)) (Utilities|Text|ToText(Integer) _output_get))
  (CameraShakes|StartCameraShake (Variables|/Script/Engine.PlayerController|GetPlayerCameraManager (Game|GetPlayerController 0)) "/Game/Blueprints/BP_Camera_Shake.BP_Camera_Shake_C" 1.0 "CameraLocal" "0, 0, 0")
  (Actor|DestroyActor)
  (if (< _output_get 1)
    (Variables|/Game/InfiniteMatrix/Blueprints/BP_Player.BP_Player_C|SetIsDead _asbp_player (< _output_get 1))
    (Default|DisplayRestart _asbp_player)))

(event EventBeginPlay
  (Utilities|FlowControl|Delay 3.0)
  (Actor|DestroyActor))

(event Collision|EventActorBeginOverlap
  (params (OtherActor :type Actor%20Object%20Reference)))

(event EventTick
  (params (DeltaSeconds :type Float%20%28single-precision%29)))

(fn ConstructionScript)