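; BP_Bullet is a player projectile that kills enemies and awards score on hit.
; Each tick it sweeps along world X at twice the player's forward speed, and it destroys itself three seconds after spawning.
; When its component hits a BP_Enemy, it destroys that enemy, increments the player's score, updates the score widget text and removes itself.
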(event OnComponentHit(Bullet)
  (params (HitComponent :type Primitive%20Component%20Object%20Reference) (OtherActor :type Actor%20Object%20Reference) (OtherComp :type Primitive%20Component%20Object%20Reference) (NormalImpulse :type Vector :default "0, 0, 0") (Hit :type Hit%20Result%20Structure%20%28by%20ref%29))
  (bind _bullet_player (Variables|Default|GetBullet_Player))
  (bind _asbp_enemy (Utilities|Casting|CastToBP_Enemy OtherActor))
  (Components|DestroyComponent (Variables|/Game/Blueprints/BP_Enemy.BP_Enemy_C|GetEnemy _asbp_enemy))
  (Actor|DestroyActor _asbp_enemy)
  (bind _output_get (Variables|/Game/InfiniteMatrix/Blueprints/BP_Player.BP_Player_C|SetScoreValue _bullet_player (+ 1 (Variables|/Game/InfiniteMatrix/Blueprints/BP_Player.BP_Player_C|GetScoreValue _bullet_player))))
  (Rendering|Components|TextRender|SetText (Variables|/Game/InfiniteMatrix/UI/WBP_Score.WBP_Score_C|GetScore (Variables|/Game/InfiniteMatrix/Blueprints/BP_Player.BP_Player_C|GetScoreWidget _bullet_player)) (Utilities|Text|ToText(Integer) _output_get))
  (Actor|DestroyActor))

(event EventBeginPlay
  (Utilities|FlowControl|Delay 3.0)
  (Actor|DestroyActor))

(event Collision|EventActorBeginOverlap
  (params (OtherActor :type Actor%20Object%20Reference)))

(event EventTick
  (params (DeltaSeconds :type Float%20%28single-precision%29))
  (Transformation|AddActorWorldOffset (Math|Vector|MakeVector (* (* (Variables|/Game/InfiniteMatrix/Blueprints/BP_Player.BP_Player_C|GetForwardSpeed (Variables|Default|GetBullet_Player)) 2.0) DeltaSeconds) 0.0 0.0) true))

(fn ConstructionScript)